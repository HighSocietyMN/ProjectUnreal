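; BP_HttpActor is an Actor with logic to load a saved WAV file for playback, with no HTTP calls despite its name.
; CustomEvent creates a MediaPlayer, opens Saved/test.WAV under the project directory, assigns it to MediaSound and prints the result.
; Nothing in the graph triggers it: BeginPlay and PlayMediaSound are empty, and the timer bound to CustomEvent is disconnected.
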(event Custom|CustomEvent
  (bind _returnvalue (Game|ConstructObjectfromClass self "/Script/MediaAssets.MediaPlayer"))
  (bind _output_get (Variables|Default|SetMedia%20Player _returnvalue))
  (bind _returnvalue_2 (Class|MediaPlayer|OpenFile _output_get (Utilities|String|Append (Class|KismetSystemLibrary|GetProjectDirectory) "Saved/test.WAV")))
  (if _returnvalue_2
    (Media|MediaSoundComponent|SetMediaPlayer (Variables|Default|GetMediaSound) (Variables|Default|GetMedia%20Player))
    (Development|PrintString "Hello End")
    (else
      (Development|PrintString "Cant Open File" true true "(R=0.000000,G=0.660000,B=1.000000,A=1.000000)" 1e+01))))

(event EventPlayMediaSound)

(event Collision|EventActorBeginOverlap
  (params (OtherActor :type Actor%20Object%20Reference)))

(event EventTick
  (params (DeltaSeconds :type Float%20%28single-precision%29)))

(event EventBeginPlay)

(fn ConstructionScript)