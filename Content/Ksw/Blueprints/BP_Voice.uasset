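; BP_Voice runs a Korean speech-to-text test on BeginPlay, printing recognized text segments and errors to the screen.
; It starts a streaming speech recognizer, then records from an audio input device for a fixed few seconds via a capturable sound wave.
; Each captured PCM chunk feeds the recognizer, and pending audio is flushed when capture stops.
; Recognition stops and the recognizer is released once it finishes with capture inactive.
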(event Custom|OnStartSpeechRecognition_Event
  (params (bSucceeded :type Boolean))
  (bind _returnvalue (Class|CapturableSoundWave|CreateCapturableSoundWave))
  (bind _output_get (Variables|Default|SetCapturableSoundWave _returnvalue))
  (EventDispatchers|BindEventtoOnPopulateAudioData _output_get (delegate Custom|OnPopulateAudioData_Event))
  (Class|CapturableSoundWave|StartCapture (Variables|Default|GetCapturableSoundWave))
  (Utilities|FlowControl|Delay 5.5)
  (Class|CapturableSoundWave|StopCapture (Variables|Default|GetCapturableSoundWave))
  (Class|SpeechRecognizer|ForceProcessPendingAudioData (Variables|Default|GetSpeechRecognizer)))

(event Custom|OnRecognitionFinished_Event
  (if (not (Class|CapturableSoundWave|IsCapturing (Variables|Default|GetCapturableSoundWave)))
    (Class|SpeechRecognizer|StopSpeechRecognition (Variables|Default|GetSpeechRecognizer))
    (Variables|Default|SetSpeechRecognizer 0)))

(event Custom|OnRecognitionError_Event
  (params (ShortErrorMessage :type String) (LongErrorMessage :type String))
  (Development|PrintString LongErrorMessage true true "(R=1.000000,G=0.000000,B=0.000000,A=1.000000)" 15.0))

(event Custom|OnRecognizedTextSegment_Event
  (params (RecognizedWords :type String))
  (Development|PrintString RecognizedWords true true "(R=0.000000,G=0.660000,B=1.000000,A=1.000000)" 12.0))

(event Custom|OnPopulateAudioData_Event
  (params (PopulatedAudioData :type Array%20of%20Floats%20%28single-precision%29))
  (bind _capturablesoundwave (Variables|Default|GetCapturableSoundWave))
  (Class|SpeechRecognizer|ProcessAudioData (Variables|Default|GetSpeechRecognizer) PopulatedAudioData (Math|Conversions|ToFloat(Integer) (Class|ImportedSoundWave|GetSampleRate _capturablesoundwave)) (Class|ImportedSoundWave|GetNumOfChannels _capturablesoundwave) true))

(event EventBeginPlay
  (bind _returnvalue (Class|SpeechRecognizer|CreateSpeechRecognizer))
  (bind _output_get (Variables|Default|SetSpeechRecognizer _returnvalue))
  (EventDispatchers|BindEventtoOnRecognitionFinished _output_get (delegate Custom|OnRecognitionFinished_Event))
  (EventDispatchers|BindEventtoOnRecognitionError (Variables|Default|GetSpeechRecognizer) (delegate Custom|OnRecognitionError_Event))
  (EventDispatchers|BindEventtoOnRecognizedTextSegment (Variables|Default|GetSpeechRecognizer) (delegate Custom|OnRecognizedTextSegment_Event))
  (Class|SpeechRecognizer|SetStreamingDefaults (Variables|Default|GetSpeechRecognizer))
  (Class|SpeechRecognizer|SetLanguage (Variables|Default|GetSpeechRecognizer) "Ko")
  (Class|SpeechRecognizer|StartSpeechRecognition (Variables|Default|GetSpeechRecognizer) (delegate Custom|OnStartSpeechRecognition_Event)))

(fn ConstructionScript)