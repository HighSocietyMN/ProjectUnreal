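; Player character Blueprint for talking to Convai AI chatbot characters by voice (hold T) or text (Enter).
; Once locally controlled, it creates chat and mic settings (F10) widgets and binds every chatbot's text, transcription and failure events to chat bubbles.
; Without a given chatbot, it targets the looked-at character within range.
; It registers itself as the environment's main character, then sends through ConvaiPlayer, optionally via the server for multiplayer.
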(event OnComponentActivated(Mesh)
  (params (Component :type Actor%20Component%20Object%20Reference) (bReset :type Boolean))
  ;[0 0 0] Begin play
  ;;[0 0 0] For multiplayer
  (Class|ActorComponent|SetIsReplicated (Variables|Default|GetConvaiPlayer) true)
  ;;[0 0 0] Ensure we are controlled by the player
  (Utilities|IsValid (Pawn|GetController) :!label _label
    (:Is%20Valid
      (if (Pawn|IsLocallyControlled)
        ;;[0 0 0] Ensure Chat widget is invalid
        (Variables|Convai|UI|SetChat_WB 0)
        ;;[0 0 0] On Start: setup the chat widget and settings menu
        (CallFunction|SetupChatWidget)
        (CallFunction|SetupSettingsWidget)))
    (:Is%20Not%20Valid
      (Utilities|FlowControl|Delay 0.2)
      (goto _label))))

(event Custom|Setup%20Chat%20Widget
  ;[0 0 0] Chat Widget
  (|SetupChatWidget))

(event Custom|Show/Hide%20Settings%20Widget
  ;[0 0 0] Settings Widget
  (|ToggleSettingsWidgetVisibility))

(event Custom|Setup%20Settings%20Widget
  ;[0 0 0] Settings Widget
  (|SetupSettingsWidget))

(event Custom|Bind%20Character%20events
  (params (Character :type Convai%20Chatbot%20Component%20Object%20Reference))
  ;[0 0 0] Chat Widget
  (|CollapseGraph Character))

(event Custom|Start%20Talking
  (params (Chatbot :type Convai%20Chatbot%20Component%20Object%20Reference))
  ;[0 0 0] Voice Interaction
  (|Talking))

(event Custom|Stop%20Talking
  ;[0 0 0] Voice Interaction
  (|Talking) ; enters at Finish Talking
)

(event Custom|Start%20Typing
  (params (ChatbotToTalkTo :type Convai%20Chatbot%20Component%20Object%20Reference))
  ;[0 0 0] Text Interaction
  (|CollapseGraph_0 ChatbotToTalkTo))

(event Input|KeyboardEvents|T
  (params (Key :type Key%20Structure :default "None"))
  ;[0 0 0] - Hold T to talk
  ; - Press Enter to Type
  ; - F10 to Open Settings
  (:Pressed
    (if (Variables|Convai|UI|GetEnablePushToTalk)
      (CallFunction|StartTalking)))
  (:Released
    (CallFunction|StopTalking)))

(event Input|KeyboardEvents|F10
  (params (Key :type Key%20Structure :default "None"))
  ;[0 0 0] - Hold T to talk
  ; - Press Enter to Type
  ; - F10 to Open Settings
  (:Pressed
    (CallFunction|Show/HideSettingsWidget)))

(event Input|KeyboardEvents|Enter
  (params (Key :type Key%20Structure :default "None"))
  ;[0 0 0] - Hold T to talk
  ; - Press Enter to Type
  ; - F10 to Open Settings
  (:Pressed
    (CallFunction|StartTyping)))

(fn ConstructionScript)

(fn FUpdateMainCharacterinEnvironment
  ;[0 0.2712 1] Set self as the main character talking to the chatbot
  (Class|ConvaiEnvironment|SetMainCharacter (Variables|/Script/Convai.ConvaiChatbotComponent|GetEnvironment (Variables|컴포넌트|GetChatbot)) (Utilities|Struct|MakeConvaiObjectEntry self "0.000000,0.000000,0.000000" "Player" "")))

(event Custom|OnTextReceivedEvent_V2_Event_0
  (params (ChatbotComponent :type Convai%20Chatbot%20Component%20Object%20Reference) (InteractingPlayerComponent :type Convai%20Player%20Component%20Object%20Reference) (CharacterName :type String) (BotText :type String) (AudioDuration :type Float%20%28single-precision%29) (IsFinal :type Boolean))
  ;[0.1834 1 0] Bind the events needed to show the chat bubbles
  (Utilities|IsValid (Variables|Convai|UI|GetChat_WB)
    (:Is%20Valid
      (Default|AddorUpdateNewChatBubble (Variables|Convai|UI|GetChat_WB) CharacterName BotText (Utilities|Struct|MakeSlateColor "(R=0.000000,G=1.000000,B=0.254000,A=1.000000)") false false IsFinal false false))))

(event Custom|ShowInChatError
  ;[1 0 0] In case a failure happened
  (Utilities|IsValid (Variables|Convai|UI|GetChat_WB)
    (:Is%20Valid
      (Default|AddorUpdateNewChatBubble (Variables|Convai|UI|GetChat_WB) "-" (Utilities|String|SelectString "Error! Contact support or check logs." "Error! See logs in Window->Output Log." (Class|KismetSystemLibrary|IsPackagedforDistribution)) (Utilities|Struct|MakeSlateColor "(R=1.000000,G=1.000000,B=0.000000,A=1.000000)") false false true false false))))

(event Custom|OnTranscriptionReceivedEvent_V2_Event_0
  (params (ChatbotComponent :type Convai%20Chatbot%20Component%20Object%20Reference) (InteractingPlayerComponent :type Convai%20Player%20Component%20Object%20Reference) (PlayerName :type String) (Transcription :type String) (IsTranscriptionReady :type Boolean) (IsFinal :type Boolean))
  ;[0.1834 1 0] Bind the events needed to show the chat bubbles
  (Utilities|IsValid InteractingPlayerComponent
    (:Is%20Valid
      (if (not (Utilities|Array|IsEmpty PlayerName))
        (Utilities|IsValid (Variables|Convai|UI|GetChat_WB)
          (:Is%20Valid
            (Default|AddorUpdateNewChatBubble (Variables|Convai|UI|GetChat_WB) PlayerName Transcription (Utilities|Struct|MakeSlateColor "(R=1.000000,G=0.250000,B=1.000000,A=1.000000)") true IsTranscriptionReady IsFinal true false)))))))

(event Custom|ShowInChatPlayer
  (params (Transcription :type String) (IsTranscriptionReady :type Boolean) (IsFinal :type Boolean))
  ;[0 0.04606 1] Deprecated Event: Not removed for backward compatability
  (Utilities|IsValid (Variables|Convai|UI|GetChat_WB)
    (:Is%20Valid
      (Default|AddorUpdateNewChatBubble (Variables|Convai|UI|GetChat_WB) (Variables|/Script/Convai.ConvaiPlayerComponent|GetPlayerName (Variables|Default|GetConvaiPlayer)) Transcription (Utilities|Struct|MakeSlateColor "(R=1.000000,G=0.250000,B=1.000000,A=1.000000)") IsTranscriptionReady true IsFinal true false))))

(event Custom|SendTextDispatcher_Event
  (params (SendText :type String))
  (bind _chatbot (Variables|컴포넌트|GetChatbot))
  (Input|SetInputModeGameOnly (Game|GetPlayerController 0) false)
  (Utilities|IsValid (Variables|Convai|UI|GetChat_WB)
    (:Is%20Valid
      (Variables|/ConvAI/Widgets/Chat_WB.Chat_WB_C|SetShowSB_SendText (Variables|Convai|UI|GetChat_WB) false)
      (CallFunction|FUpdateMainCharacterinEnvironment)
      ;[1 1 1] Send text to the character
      (Class|ConvaiPlayerComponent|SendText (Variables|Default|GetConvaiPlayer) _chatbot SendText (Variables|/Script/Convai.ConvaiChatbotComponent|GetEnvironment _chatbot) true true (Variables|Convai|Multiplayer|GetEnable%20Multiplayer) (Variables|Convai|Multiplayer|GetUse%20Server%20API%20Key))
      ;[1 1 1] Make sure the chat widget is set with this character
      (CallFunction|BindCharacterEvents (Variables|컴포넌트|GetChatbot)))))

(event Custom|Done%20Pressed_Event_0
  (params (PlayerName :type String) (UISelection :type Integer) (UseServerAPI_Key :type Boolean))
  (Utilities|FlowControl|Sequence
    (:then_0
      (CallFunction|Show/HideSettingsWidget))
    (:then_1
      (if (Utilities|Enum|NotEqual(Enum) PlayerName "")
        (Variables|/Script/Convai.ConvaiPlayerComponent|SetPlayerName (Variables|Default|GetConvaiPlayer) PlayerName)))
    (:then_2
      (bind _output_get (Variables|Convai|UI|SetUISelection UISelection))
      (Default|FUISelection (Variables|Convai|UI|GetChat_WB) _output_get))
    (:then_3
      (Variables|Convai|Multiplayer|SetUse%20Server%20API%20Key UseServerAPI_Key))))